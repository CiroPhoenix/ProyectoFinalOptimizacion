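; Enemy spawner actor that produces recurring waves of a configurable enemy class for as long as it runs.
; From BeginPlay, a custom event spawns the set number of enemies in one loop, all at the spawner's transform.
; It then waits for the spawn delay and calls itself again with the current transform, repeating with no stop condition or cap on live enemies.
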(event `self.ReceiveBeginPlay`
  (`self.SpawnEnemies` (`self.Enemy`) (`self.GetTransform`) (`self.Number Of Enemies`)))

(event `SpawnEnemies`
  (params (Enemy :type "Actor Class Reference") (SpawnTransform :type "Transform Structure") (`NumberOf Enemies` :type Integer))
  (for _ (range `NumberOf Enemies`)
    (`|SpawnActorFromClass` Enemy SpawnTransform "Undefined" "OverrideRootScale" null null))
  (`KismetSystemLibrary.Delay` (`self.Spawn Delay`))
  (`self.SpawnEnemies` (`self.Enemy`) (`self.GetTransform`) (`self.Number Of Enemies`)))

(fn `UserConstructionScript`)