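; Melee enemy character that chases the player, deals damage on reaching them and can be killed.
; On BeginPlay it picks a random walk speed and starts ChasePlayer, which re-calls itself after each AI MoveTo success or failure.
; AnyDamage lowers Health, pausing movement for a random hit montage.
; At zero Health it plays a random death montage, disables capsule collision and destroys itself after a delay.
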(event `self.ReceiveAnyDamage`
  (params (Damage :type "Float (single-precision)") (DamageType :type "DamageType Object Reference") (InstigatedBy :type "Controller Object Reference") (DamageCauser :type "Actor Object Reference"))
  (if (not (`self.Death?`))
    (bind _output_get (set `self.Health` (`KismetMathLibrary.FClamp` (- (`self.Health`) Damage) 0.0 100.0)))
    (if (== _output_get 0.0)
      (`CharacterMovementComponent.DisableMovement` (`self.CharacterMovement`))
      (set `self.Death?` true)
      (`self.PlayAnimMontage` (select `int` (`KismetMathLibrary.RandomInteger` 3) :`0` "/Game/EnemigosMaterial/Animaciones/DamageAndDead/Death_1_Montage.Death_1_Montage" :`1` "/Game/EnemigosMaterial/Animaciones/DamageAndDead/Death_2_Montage.Death_2_Montage" :`2` "/Game/EnemigosMaterial/Animaciones/DamageAndDead/Death_3_Montage.Death_3_Montage" :`3` "/Game/EnemigosMaterial/Animaciones/DamageAndDead/Death_4_Montage.Death_4_Montage" :!type "AnimMontage Object Reference"))
      (`PrimitiveComponent.SetCollisionEnabled` (`self.CapsuleComponent`) "NoCollision")
      (`KismetSystemLibrary.Delay` 15.0)
      (`self.K2_DestroyActor`)
      (else
        (`CharacterMovementComponent.DisableMovement` (`self.CharacterMovement`))
        (bind _returnvalue (`self.PlayAnimMontage` (select `int` (`KismetMathLibrary.RandomInteger` 3) :`0` "/Game/EnemigosMaterial/Animaciones/DamageAndDead/Hit_1_Montage.Hit_1_Montage" :`1` "/Game/EnemigosMaterial/Animaciones/DamageAndDead/Hit_2_Montage.Hit_2_Montage" :`2` "/Game/EnemigosMaterial/Animaciones/DamageAndDead/Hit_3_Montage.Hit_3_Montage" :`3` "/Game/EnemigosMaterial/Animaciones/DamageAndDead/Hit_4_Montage.Hit_4_Montage" :!type "AnimMontage Object Reference")))
        (`KismetSystemLibrary.Delay` _returnvalue)
        (if (not (`self.Death?`))
          (`CharacterMovementComponent.SetMovementMode` (`self.CharacterMovement`) "MOVE_Walking" 0))))))

(event `self.ReceiveBeginPlay`
  (bind _asthird_person_character (cast `/Game/ThirdPersonBP/Blueprints/ThirdPersonCharacter` (`GameplayStatics.GetPlayerCharacter` 0)))
  (bind _output_get (set `self.Char Ref` _asthird_person_character))
  (`self.Chase Player` _output_get)
  (set `CharacterMovementComponent.MaxWalkSpeed` (select `int` (`KismetMathLibrary.RandomInteger` 4) :`0` 200.0 :`1` 250.0 :`2` 300.0 :`3` 350.0 :`4` 400.0 :!type "Float (single-precision)") (`self.CharacterMovement`)))

(event `Chase Player`
  (params (PlayerToChase :type "/Game/ThirdPersonBP/Blueprints/ThirdPersonCharacter Object Reference"))
  (if (not (`self.Death?`))
    (`|AIMoveTo` self (0.0 0.0 0.0) PlayerToChase
      (:`OnSuccess`
        (if true
          (`GameplayStatics.ApplyDamage` (`self.Char Ref`) (`self.Damage`))
          (`self.Chase Player` (`self.Char Ref`) :!label _label)))
      (:`OnFail`
        (if true
          (goto _label))))))

(fn `UserConstructionScript`)