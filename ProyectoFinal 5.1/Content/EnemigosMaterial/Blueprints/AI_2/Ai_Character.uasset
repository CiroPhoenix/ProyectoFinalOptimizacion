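; Enemy AI character that roams, patrols between two target points or chases the player, as set by its AIState.
; PawnSensing switches it to chasing on sight: it moves to the player, applies delayed damage and repeats with randomized walk speeds.
; Incoming damage plays random hit montages that pause movement, or at zero health a death montage and sound before delayed destruction.
; The player's death event re-enables sensing and restarts the configured state.
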(event `Reset_AI`
  ;[1 1 1] Select state
  (`PawnSensingComponent.SetSensingUpdatesEnabled` (`self.PawnSensing`) true)
  (switch `/Game/EnemigosMaterial/Blueprints/AI_2/E_AI_State` (`self.AI_State`)
    (:`NewEnumerator1`
      (`self.Roam`))
    (:`NewEnumerator2`
      (`self.ChasePlayer` null))
    (:`NewEnumerator3`
      (`self.Patrol`))))

(event `self.ReceiveBeginPlay`
  ;[1 1 1] Select state
  (bind _asthird_person_character (cast `/Game/ThirdPersonBP/Blueprints/ThirdPersonCharacter` (`GameplayStatics.GetPlayerCharacter` 0)))
  (add `/Game/ThirdPersonBP/Blueprints/ThirdPersonCharacter.PlayerDied` _asthird_person_character (delegate `Reset_AI`))
  (switch `/Game/EnemigosMaterial/Blueprints/AI_2/E_AI_State` (`self.AI_State`)
    (:`NewEnumerator1`
      (`self.Roam`))
    (:`NewEnumerator2`
      (`self.ChasePlayer` null))
    (:`NewEnumerator3`
      (`self.Patrol`))))

(event `Roam`
  ;[1 1 1] Roam
  (`|AIMoveTo` self (`NavigationSystemV1.K2_GetRandomLocationInNavigableRadius` (`self.K2_GetActorLocation`) 500.0 null null) null
    (:`OnSuccess`
      (`KismetSystemLibrary.Delay` 1.0)
      (`self.Roam`))))

(event `ChasePlayer`
  (params (PlayerToChase :type "Pawn Object Reference"))
  ;[1 1 1] Chase player
  (if (not (`self.DeathAI?`))
    (`|AIMoveTo` self (0.0 0.0 0.0) PlayerToChase
      (:`OnSuccess`
        (`KismetSystemLibrary.Delay` 0.9)
        (if (not (`self.DeathAI?`))
          (`GameplayStatics.ApplyDamage` PlayerToChase (`self.Damage`))
          (`KismetSystemLibrary.Delay` 2.0)
          (`self.ChasePlayer` PlayerToChase)
          (set `CharacterMovementComponent.MaxWalkSpeed` (select `int` (`KismetMathLibrary.RandomInteger` 4) :`0` 250.0 :`1` 300.0 :`2` 350.0 :`3` 400.0 :`4` 450.0 :!type "Float (single-precision)") (`self.CharacterMovement`)))))))

(event `Patrol`
  ;[1 1 1] Patrol
  (`|AIMoveTo` self (0.0 0.0 0.0) (`self.TargetPoint1`)
    (:`OnSuccess`
      (`KismetSystemLibrary.Delay` 3.0)
      (`|AIMoveTo` self (0.0 0.0 0.0) (`self.TargetPoint2`)
        (:`OnSuccess`
          (`KismetSystemLibrary.Delay` 3.0)
          (`self.Patrol`))))))

(event `self.ReceiveAnyDamage`
  (params (Damage :type "Float (single-precision)") (DamageType :type "DamageType Object Reference") (InstigatedBy :type "Controller Object Reference") (DamageCauser :type "Actor Object Reference"))
  ;[1 1 1] Make Damage to AI
  (if (not (`self.DeathAI?`))
    (bind _output_get (set `self.AI_Health` (`KismetMathLibrary.FClamp` (- (`self.AI_Health`) Damage) 0.0 100.0)))
    (if (== _output_get 0.0)
      (`CharacterMovementComponent.DisableMovement` (`self.CharacterMovement`))
      (set `self.DeathAI?` true)
      (`GameplayStatics.SpawnSound2D` "/Game/SoundEffects/DeathEnemySounds/DeathSoundCue.DeathSoundCue" 1.0 1.0 0.0 null)
      (`self.PlayAnimMontage` (select `int` (`KismetMathLibrary.RandomInteger` 3) :`0` "/Game/EnemigosMaterial/Animaciones/DamageAndDead/Death_1_Montage.Death_1_Montage" :`1` "/Game/EnemigosMaterial/Animaciones/DamageAndDead/Death_2_Montage.Death_2_Montage" :`2` "/Game/EnemigosMaterial/Animaciones/DamageAndDead/Death_3_Montage.Death_3_Montage" :`3` "/Game/EnemigosMaterial/Animaciones/DamageAndDead/Death_4_Montage.Death_4_Montage" :!type "AnimMontage Object Reference"))
      (`PrimitiveComponent.SetCollisionEnabled` (`self.CapsuleComponent`) "NoCollision")
      (`KismetSystemLibrary.Delay` 20.0)
      (`self.K2_DestroyActor`)
      (else
        (`CharacterMovementComponent.DisableMovement` (`self.CharacterMovement`))
        (bind _returnvalue (`self.PlayAnimMontage` (select `int` (`KismetMathLibrary.RandomInteger` 3) :`0` "/Game/EnemigosMaterial/Animaciones/DamageAndDead/Hit_1_Montage.Hit_1_Montage" :`1` "/Game/EnemigosMaterial/Animaciones/DamageAndDead/Hit_2_Montage.Hit_2_Montage" :`2` "/Game/EnemigosMaterial/Animaciones/DamageAndDead/Hit_3_Montage.Hit_3_Montage" :`3` "/Game/EnemigosMaterial/Animaciones/DamageAndDead/Hit_4_Montage.Hit_4_Montage" :!type "AnimMontage Object Reference")))
        (`KismetSystemLibrary.Delay` _returnvalue)
        (if (not (`self.DeathAI?`))
          (`CharacterMovementComponent.SetMovementMode` (`self.CharacterMovement`) "MOVE_Walking" 0))))))

(event `self.PawnSensing.OnSeePawn`
  (params (Pawn :type "Pawn Object Reference"))
  ;[1 1 1] Chase player when we see the them
  (bind _asthird_person_character (cast `/Game/ThirdPersonBP/Blueprints/ThirdPersonCharacter` Pawn))
  (`self.ChasePlayer` _asthird_person_character))

(fn `UserConstructionScript`)