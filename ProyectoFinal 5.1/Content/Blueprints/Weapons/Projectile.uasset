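; Projectile Blueprint that damages what it hits and destroys itself, provided the hit component simulates physics, queried with "Enemy" as the bone name.
; A sequence first applies a velocity-based force scaled to zero and destroys the actor, then applies randomly selected damage and destroys again.
; The random index never reaches the last damage option, and an impulse variant of the push is left unconnected.
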(event `self.ReceiveHit`
  (params (MyComp :type "PrimitiveComponent Object Reference") (Other :type "Actor Object Reference") (OtherComp :type "PrimitiveComponent Object Reference") (bSelfMoved :type Boolean) (HitLocation :type "Vector Structure") (HitNormal :type "Vector Structure") (NormalImpulse :type "Vector Structure") (Hit :type "HitResult Structure (by ref)"))
  (if (`SceneComponent.IsSimulatingPhysics` OtherComp "Enemy")
    (`|ExecutionSequence`
      (:`then_0`
        (`PrimitiveComponent.AddForceAtLocation` OtherComp (* (`self.GetVelocity`) 0.0) (`self.K2_GetActorLocation`) "None")
        (`self.K2_DestroyActor`))
      (:`then_1`
        (`GameplayStatics.ApplyDamage` Other (select `int` (`KismetMathLibrary.RandomInteger` 3) :`0` 10.0 :`1` 20.0 :`2` 30.0 :`3` 15.0 :!type "Float (single-precision)") null self)
        (`self.K2_DestroyActor`)))))

(fn `UserConstructionScript`)